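; VR player Blueprint with floor-origin tracking, hands that follow the motion controllers, and a sonar post-process effect driven by werewolf positions.
; Each Tick rebuilds the camera's blendables, creating a new dynamic sonar material for every BP_Werewolf and feeding it that enemy's location.
; Right-controller overlaps call HandleCollision and play a hit sound at the player's location.
; The Death_Button input only tracks its held state in ButtonPressed.
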(event OnComponentBeginOverlap(RightController)
  (params (OverlappedComponent :type Primitive%20Component%20Object%20Reference) (OtherActor :type Actor%20Object%20Reference) (OtherComp :type Primitive%20Component%20Object%20Reference) (OtherBodyIndex :type Integer) (bFromSweep :type Boolean) (SweepResult :type Hit%20Result%20Structure%20%28by%20ref%29))
  (Class|VRPlayer|HandleCollision OtherComp)
  (Audio|PlaySoundatLocation "/Game/Sound/Sword/Treffer.Treffer" (Transformation|GetActorLocation) "0, 0, 0" 1.0 1.0 0.0 0 0 0))

(event EventTick
  (params (DeltaSeconds :type Float%20%28single-precision%29))
  (Transformation|SetRelativeTransform (Variables|Default|GetLeftHand) (Transformation|GetRelativeTransform (Variables|Default|GetLeftController)) false false)
  (Transformation|SetRelativeTransform (Variables|Default|GetRightHand) (Transformation|GetRelativeTransform (Variables|Default|GetRightController)) false false)
  (Utilities|Array|Clear (Variables|Default|GetWheightedBlendables))
  (bind _outactors (Actor|GetAllActorsOfClass "/Game/Characters/Werewolf/BP_Werewolf.BP_Werewolf_C"))
  (for _array_element _outactors
    (bind _returnvalue (Rendering|Material|CreateDynamicMaterialInstance "/Game/Materials/MI_Sonar.MI_Sonar" "None" :!class /Script/Engine.KismetMaterialLibrary))
    (Rendering|Material|SetVectorParameterValue _returnvalue "EnemyLocation" (Math|Conversions|ToLinearColor(Vector) (Transformation|GetActorLocation _array_element)) :!class /Script/Engine.MaterialInstanceDynamic)
    (Utilities|Array|Add (Variables|Default|GetWheightedBlendables) (Utilities|Struct|MakeWeightedBlendable 1.0 _returnvalue)))
  (Variables|/Script/Engine.CameraComponent|SetPostProcessSettings (Variables|Default|GetCamera) (Utilities|Struct|MakePostProcessSettings (Utilities|Struct|MakeWeightedBlendables (Variables|Default|GetWheightedBlendables)))))

(event EventBeginPlay
  (Class|HeadMountedDisplayFunctionLibrary|SetTrackingOrigin "Floor"))

(event Input|ActionEvents|InputActionDeath_Button
  (params (Key :type Key%20Structure))
  (:Pressed
    (Variables|Default|SetButtonPressed true))
  (:Released
    (Variables|Default|SetButtonPressed false)))

(fn ConstructionScript)