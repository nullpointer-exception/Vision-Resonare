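; BP_FPVPlayer is the first-person player character, handling movement, look input and a simple attack pose.
; Move axes add movement input along the control rotation's yaw only, while Turn and LookUp drive controller yaw and pitch.
; MouseAttack nudges and rotates the VisusProp component on press and applies the opposite offset on release, with no hit or damage logic.
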(event EventBeginPlay)

(event Collision|EventActorBeginOverlap
  (params (OtherActor :type Actor%20Object%20Reference)))

(event EventTick
  (params (DeltaSeconds :type Float%20%28single-precision%29)))

(event Input|ActionEvents|InputActionMouseAttack
  (params (Key :type Key%20Structure :default "None"))
  (bind _visusprop (Variables|Default|GetVisusProp))
  (:Pressed
    (Class|SceneComponent|AddLocalTransform _visusprop (Math|Transform|MakeTransform "5.000000, 0, 0" "0, 0,45.000000") false false))
  (:Released
    (Class|SceneComponent|AddLocalTransform _visusprop (Math|Transform|MakeTransform "-5.000000, 0, 0" "0, 0,-45.000000") false false)))

(event Input|AxisEvents|InputAxisMoveForward
  (params (AxisValue :type Float%20%28single-precision%29))
  ;[1 1 1] Movement FPV (PK)
  (Pawn|Input|AddMovementInput (Math|Vector|GetForwardVector (Math|Rotator|MakeRotator 0.0 0.0 (.Yaw (Math|Rotator|BreakRotator (Pawn|GetControlRotation :!class /Script/Engine.Pawn))))) AxisValue false))

(event Input|AxisEvents|InputAxisMoveRight
  (params (AxisValue :type Float%20%28single-precision%29))
  ;[1 1 1] Movement FPV (PK)
  (Pawn|Input|AddMovementInput (Math|Vector|GetRightVector (Math|Rotator|MakeRotator 0.0 0.0 (.Yaw (Math|Rotator|BreakRotator (Pawn|GetControlRotation :!class /Script/Engine.Pawn))))) AxisValue false))

(event Input|AxisEvents|InputAxisTurn
  (params (AxisValue :type Float%20%28single-precision%29))
  (Pawn|Input|AddControllerYawInput AxisValue))

(event Input|AxisEvents|InputAxisLookUp
  (params (AxisValue :type Float%20%28single-precision%29))
  (Pawn|Input|AddControllerPitchInput AxisValue))

(fn ConstructionScript)