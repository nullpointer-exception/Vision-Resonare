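; Right-hand controller actor for the VR player, handling damage to the player and hit audio for its Visus mesh.
; Capsule hits print a debug message, subtract a fixed amount from BP_VRPlayer's health and open the main menu level once it is depleted.
; Visus mesh overlaps call the empty ActorBeginOverlap event and play the Treffer sound at the location of VisusLow's owner.
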(event OnComponentHit(CapsuleComponent)
  (params (HitComponent :type Primitive%20Component%20Object%20Reference) (OtherActor :type Actor%20Object%20Reference) (OtherComp :type Primitive%20Component%20Object%20Reference) (NormalImpulse :type Vector :default "0, 0, 0") (Hit :type Hit%20Result%20Structure%20%28by%20ref%29))
  ;[1 1 1] Health System Player (by Patrick Kokoszka)
  (Development|PrintString "HIT!")
  (bind _asbp_vrplayer (Utilities|Casting|CastToBP_VRPlayer (Game|Player|GetPlayerPawn 0)))
  (Variables|/Game/Characters/Player/Blueprints/BP_VRPlayer.BP_VRPlayer_C|SetPlayerHealth _asbp_vrplayer (- (Variables|/Game/Characters/Player/Blueprints/BP_VRPlayer.BP_VRPlayer_C|GetPlayerHealth _asbp_vrplayer) 1e+02))
  (if (<= (Variables|/Game/Characters/Player/Blueprints/BP_VRPlayer.BP_VRPlayer_C|GetPlayerHealth _asbp_vrplayer) 0.0)
    (Game|OpenLevel(byName) "Mein Menu")))

(event OnComponentBeginOverlap(SM_Visus)
  (params (OverlappedComponent :type Primitive%20Component%20Object%20Reference) (OtherActor :type Actor%20Object%20Reference) (OtherComp :type Primitive%20Component%20Object%20Reference) (OtherBodyIndex :type Integer) (bFromSweep :type Boolean) (SweepResult :type Hit%20Result%20Structure%20%28by%20ref%29))
  (Class|RightController|ActorBeginOverlap OtherActor OtherActor)
  (Audio|PlaySoundatLocation "/Game/Sound/Schwert/Treffer.Treffer" (Transformation|GetActorLocation (Components|GetOwner (Variables|Default|GetVisus_low))) "0, 0, 0" 1.0 1.0 0.0 0 0 0))

(event EventBeginPlay)

(event Collision|EventActorBeginOverlap
  (params (OtherActor :type Actor%20Object%20Reference)))

(event EventTick
  (params (DeltaSeconds :type Float%20%28single-precision%29)))

(fn ConstructionScript)