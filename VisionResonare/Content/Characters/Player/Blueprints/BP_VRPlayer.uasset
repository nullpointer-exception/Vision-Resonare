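; VR player pawn with arm-swing locomotion, a looping-style heartbeat sound and health that loads StartScreen when hits deplete it.
; While both movement inputs are held, per-frame controller travel scales a swept move along the averaged horizontal controller forward vectors.
; Tick also writes the first BP_Werewolf's position to MC_Sonar for the sonar effect.
; Single-hand movement and per-enemy post-process sonar logic are present but never run.
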(event OnComponentHit(CapsuleComponent)
  (params (HitComponent :type Primitive%20Component%20Object%20Reference) (OtherActor :type Actor%20Object%20Reference) (OtherComp :type Primitive%20Component%20Object%20Reference) (NormalImpulse :type Vector :default "0, 0, 0") (Hit :type Hit%20Result%20Structure%20%28by%20ref%29))
  ;[1 1 1] Health System Player (by Patrick Kokoszka)
  (Development|PrintString "HIT!")
  (Variables|Default|SetPlayerHealth (- (Variables|Default|GetPlayerHealth) 1e+02))
  (if (<= (Variables|Default|GetPlayerHealth) 0.0)
    (Game|LoadStreamLevel(byName) "StartScreen" false)))

(event EventTick
  (params (DeltaSeconds :type Float%20%28single-precision%29))
  (CallFunction|CheckVRMovemt)
  (CallFunction|SetEnemyPosition))

(event EventBeginPlay
  (Class|HeadMountedDisplayFunctionLibrary|SetTrackingOrigin "Floor")
  (bind _returnvalue (Audio|CreateSound2D "/Game/Sound/Player/SC_Heartbeat.SC_Heartbeat" 1.0 1.0 0.0 0))
  (bind _output_get (Variables|Default|SetHeartSound _returnvalue))
  (Audio|Components|Audio|Play _output_get 0.0))

(event Input|AxisEvents|InputAxisVR_Movement_L
  (params (AxisValue :type Float%20%28single-precision%29))
  (if (!= AxisValue 0.0)
    (Variables|Default|SetisLeftActive true)
    (else
      (Variables|Default|SetisLeftActive false))))

(event Input|AxisEvents|InputAxisVR_Movement_R
  (params (AxisValue :type Float%20%28single-precision%29))
  (if (!= AxisValue 0.0)
    (Variables|Default|SetisRightActive true)
    (else
      (Variables|Default|SetisRightActive false))))

(fn ConstructionScript)

(fn SetEnemyPosition
  (bind _outactors (Actor|GetAllActorsOfClass "/Game/Characters/Werewolf/Blueprints/BP_Werewolf.BP_Werewolf_C"))
  (Utilities|IsValid (Utilities|Array|Get(acopy) _outactors)
    (:Is%20Valid
      (Rendering|Material|SetVectorParameterValue "/Game/Base/Materials/MC_Sonar.MC_Sonar" "EnemyPosition" (Math|Conversions|ToLinearColor(Vector) (Transformation|GetActorLocation (Utilities|Array|Get(acopy) _outactors))) :!class /Script/Engine.KismetMaterialLibrary))))

(fn CheckVRMovemt
  (if (and (Variables|Default|GetisLeftActive) (Variables|Default|GetisRightActive))
    (bind _distance (CallFunction|GetControllerDistance "NewEnumerator2"))
    (bind _outputvector (CallFunction|CheckControllerDirection "NewEnumerator2"))
    (CallFunction|AddPlayerMovement (* _outputvector (* _distance (Variables|Default|GetMovementSpeed)))))
  (Variables|Default|SetPreviousLeftController (Utilities|LeftControllerPosition))
  (Variables|Default|SetPreviousRightController (Utilities|RightControllerPosition)))

(fn CheckControllerDirection
  (params (InputType :type E_VR_Movement%20Enum :default "NewEnumerator0"))
  (bind _leftcontroller (Variables|Default|GetLeftController))
  (bind _rightcontroller (Variables|Default|GetRightController))
  (bind _leftcontroller_2 (Variables|Default|GetLeftController))
  (bind _rightcontroller_2 (Variables|Default|GetRightController))
  (bind _rightcontroller_3 (Variables|/Script/VisionResonare.RightController|GetRightController _rightcontroller_2))
  (bind _leftcontroller_3 (Variables|/Script/VisionResonare.LeftController|GetLeftController _leftcontroller))
  (bind _rightcontroller_4 (Variables|/Script/VisionResonare.RightController|GetRightController _rightcontroller))
  (bind _leftcontroller_4 (Variables|/Script/VisionResonare.LeftController|GetLeftController _leftcontroller_2))
  (bind _returnvalue (Math|Vector|GetForwardVector _leftcontroller_3))
  (bind _returnvalue_2 (Math|Vector|GetForwardVector _leftcontroller_4))
  (bind _returnvalue_3 (Math|Vector|GetForwardVector _rightcontroller_3))
  (bind _returnvalue_4 (Math|Vector|GetForwardVector _rightcontroller_4))
  (switch Utilities|FlowControl|Switch|SwitchonE_VR_Movement InputType
    (:NewEnumerator0
      (LocalVariables|SetOutputtingVector (Math|Vector|Normalize (Math|Vector|MakeVector (.x _returnvalue_2) (.y _returnvalue_2) 0.0))))
    (:NewEnumerator1
      (LocalVariables|SetOutputtingVector (Math|Vector|Normalize (Math|Vector|MakeVector (.x _returnvalue_3) (.y _returnvalue_3) 0.0))))
    (:NewEnumerator2
      (LocalVariables|SetOutputtingVector (/ (+ (Math|Vector|Normalize (Math|Vector|MakeVector (.x _returnvalue) (.y _returnvalue) 0.0)) (Math|Vector|Normalize (Math|Vector|MakeVector (.x _returnvalue_4) (.y _returnvalue_4) 0.0))) 2))))
  (return (LocalVariables|GetOutputtingVector)))

(fn GetControllerDistance
  (params (ControllerType :type E_VR_Movement%20Enum :default "NewEnumerator0"))
  (switch Utilities|FlowControl|Switch|SwitchonE_VR_Movement ControllerType
    (:NewEnumerator0
      (LocalVariables|SetOutputDistance (Math|Vector|VectorLength (- (Utilities|LeftControllerPosition) (Variables|Default|GetPreviousLeftController)))))
    (:NewEnumerator1
      (LocalVariables|SetOutputDistance (Math|Vector|VectorLength (- (Utilities|RightControllerPosition) (Variables|Default|GetPreviousRightController)))))
    (:NewEnumerator2
      (LocalVariables|SetOutputDistance (+ (Math|Vector|VectorLength (- (Utilities|LeftControllerPosition) (Variables|Default|GetPreviousLeftController))) (Math|Vector|VectorLength (- (Utilities|RightControllerPosition) (Variables|Default|GetPreviousRightController)))))))
  (return (LocalVariables|GetOutputDistance)))

(fn AddPlayerMovement
  (params (MovementInput :type Vector))
  (Transformation|SetActorLocation (+ (Transformation|GetActorLocation) MovementInput) true false))