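; Werewolf enemy character with melee attack, health and death handling.
; BeginPlay snaps the damage trigger to the right-hand socket, and MeleeAttack plays an attack montage.
; Capsule overlaps with a Ruptor or the FPV player's VisusProp component subtract health and loop a hit animation.
; Tick detects zero health and, once, increments the enemy spawner's counter, plays the death animation and destroys the actor after a delay.
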(event OnComponentBeginOverlap(CapsuleComponent)
  (params (OverlappedComponent :type Primitive%20Component%20Object%20Reference) (OtherActor :type Actor%20Object%20Reference) (OtherComp :type Primitive%20Component%20Object%20Reference) (OtherBodyIndex :type Integer) (bFromSweep :type Boolean) (SweepResult :type Hit%20Result%20Structure%20%28by%20ref%29))
  ;[1 1 1] Health System Werewolf (by Patrick Kokoszka)
  (if (not (Variables|Default|GetIsDead))
    (Utilities|Casting|CastToBP_Visus OtherActor
      (:CastFailed
        (Utilities|Casting|CastToBP_Ruptor OtherActor
          (:then
            (Components|Animation|PlayAnimation (Variables|Character|GetMesh) "/Game/Characters/Werewolf/Animations/Hit_Anim.Hit_Anim" true :!label _label)
            (Variables|Default|SetHealth (- (Variables|Default|GetHealth) 1e+01))
            (if (<= (Variables|Default|GetHealth) 0.0)
              (Variables|Default|SetIsDead true)))
          (:CastFailed
            (bind _asbp_fpvplayer (Utilities|Casting|CastToBP_FPVPlayer OtherActor))
            (if (== (Variables|/Game/Characters/Player/Blueprints/BP_FPVPlayer.BP_FPVPlayer_C|GetVisusProp _asbp_fpvplayer) OtherComp)
              (goto _label))))))))

(event EventBeginPlay
  (Transformation|AttachComponentToComponent (Variables|Default|GetDMGTrigger) (Variables|Character|GetMesh) "r_hand_skin_end" "SnapToTarget" "SnapToTarget" "KeepWorld" true))

(event EventTick
  (params (DeltaSeconds :type Float%20%28single-precision%29))
  (if (<= (Variables|Default|GetHealth) 0.0)
    (Variables|Default|SetIsDead true)
    (if (Variables|Default|GetIsDead)
      (Utilities|FlowControl|DoOnce false
        (:Completed
          (bind _outactors (Actor|GetAllActorsOfClass "/Game/Gameplay/BP_EnemySpawner.BP_EnemySpawner_C"))
          (bind _asbp_enemy_spawner (Utilities|Casting|CastToBP_EnemySpawner (Utilities|Array|Get(acopy) _outactors)))
          (Variables|/Game/Gameplay/BP_EnemySpawner.BP_EnemySpawner_C|SetEnemies%20Counter _asbp_enemy_spawner (+ (Variables|/Game/Gameplay/BP_EnemySpawner.BP_EnemySpawner_C|GetEnemies%20Counter _asbp_enemy_spawner) 1))
          (Components|Animation|PlayAnimation (Variables|Character|GetMesh) "/Game/Characters/Werewolf/Animations/Death_Anim.Death_Anim" false)
          (Utilities|FlowControl|Delay 2.6)
          (Actor|DestroyActor))))))

(event EventMeleeAttack
  ;[1 1 1] AttackPlayer Werewolf (by Patrick Kokoszka)
  (Animation|Montage|PlayMontage (Variables|Character|GetMesh) 0))

(event Collision|EventActorBeginOverlap
  (params (OtherActor :type Actor%20Object%20Reference))
  (if (== OtherActor self)
    _))

(fn ConstructionScript)