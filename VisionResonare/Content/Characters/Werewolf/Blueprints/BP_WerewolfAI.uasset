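; AI controller for the werewolf that starts the Werewolf_BT behavior tree on BeginPlay.
; Every tick it copies the controlled BP_Werewolf's Health into the blackboard.
; Its perception update only casts the sensed actor to BP_VRPlayer; the node that would write CanSeePlayer to the blackboard is disconnected and never runs.
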(event OnTargetPerceptionUpdated(AIPerception)
  (params (Actor :type Actor%20Object%20Reference) (Stimulus :type AI%20Stimulus%20Structure))
  ;[1 1 1] AIPerception WerewolfAI
  (Utilities|Casting|CastToBP_VRPlayer Actor))

(event EventBeginPlay
  ;[1 1 1] RunBehaviourTree WerewolfAI
  (AI|RunBehaviorTree "/Game/Characters/Werewolf/AI/Werewolf_BT.Werewolf_BT"))

(event EventTick
  (params (DeltaSeconds :type Float%20%28single-precision%29))
  ;[1 1 1] CastHealthtoBlackboard WerewolfAI
  (bind _asbp_werewolf (Utilities|Casting|CastToBP_Werewolf (Pawn|GetControlledPawn)))
  (AI|Components|Blackboard|SetValueasFloat (AI|GetBlackboard 0) (Utilities|Name|MakeLiteralName "Health") (Variables|/Game/Characters/Werewolf/Blueprints/BP_Werewolf.BP_Werewolf_C|GetHealth _asbp_werewolf)))

(fn ConstructionScript)