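; BP_VRPlayer is the VR player Blueprint, using floor-level tracking with a left and right hand.
; Every tick it copies each motion controller's relative transform onto the matching hand component, without sweep or teleport.
; Only the right controller responds to overlaps, passing the other component to HandleCollision, whose logic is not defined here.
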(event OnComponentBeginOverlap(RightController)
  (params (OverlappedComponent :type Primitive%20Component%20Object%20Reference) (OtherActor :type Actor%20Object%20Reference) (OtherComp :type Primitive%20Component%20Object%20Reference) (OtherBodyIndex :type Integer) (bFromSweep :type Boolean) (SweepResult :type Hit%20Result%20Structure%20%28by%20ref%29))
  (Class|VRPlayer|HandleCollision OtherComp))

(event EventTick
  (params (DeltaSeconds :type Float%20%28single-precision%29))
  (Transformation|SetRelativeTransform (Variables|Default|GetLeftHand) (Transformation|GetRelativeTransform (Variables|Default|GetLeftController)) false false)
  (Transformation|SetRelativeTransform (Variables|Default|GetRightHand) (Transformation|GetRelativeTransform (Variables|Default|GetRightController)) false false))

(event EventBeginPlay
  (Class|HeadMountedDisplayFunctionLibrary|SetTrackingOrigin "Floor"))

(fn ConstructionScript)