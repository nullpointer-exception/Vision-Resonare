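; BP_RandomTrees is a landscape Blueprint that scatters trees with branches around its origin during construction.
; For each of Amount iterations, TreeSpawner adds an instanced static mesh component at a random XY offset scaled by Range, with Z at zero.
; BranchSpawner adds a second component at that same relative location.
; Placement uses no seed, so the layout re-randomizes whenever the construction script reruns.
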(fn ConstructionScript
  (for _index (range 1 (Variables|Default|GetAmount))
    (bind _relative_location (CallFunction|TreeSpawner))
    (CallFunction|BranchSpawner _relative_location)))

(fn TreeSpawner
  (bind _returnvalue (Math|Random|RandomUnitVector))
  (bind _range (Variables|Default|GetRange))
  (bind _returnvalue_2 (* _returnvalue _range))
  (bind (_x _y) (Math|Vector|BreakVector _returnvalue_2))
  (bind _returnvalue_3 (AddComponent|AddInstancedStaticMeshComponent false (Math|Conversions|ToTransform(Vector) (Math|Vector|MakeVector _x _y 0.0))))
  (return (Variables|/Script/Engine.SceneComponent|GetRelativeLocation _returnvalue_3)))

(fn BranchSpawner
  (params (Relative%20Loaction :type Vector))
  (AddComponent|AddInstancedStaticMeshComponent false (Math|Conversions|ToTransform(Vector) Relative%20Loaction)))