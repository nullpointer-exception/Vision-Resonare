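; Portcullis gate that moves vertically when something enters its trigger box and closes once the box is empty.
; A counter tracks overlaps, and a DoOnce stops the open animation restarting until the last occupant leaves.
; Separate open and close timelines set the mesh's absolute world Z from their curve, a direction multiplier and Height, rather than offsetting from its placed position.
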(event OnComponentBeginOverlap(Box)
  (params (OverlappedComponent :type Primitive%20Component%20Object%20Reference) (OtherActor :type Actor%20Object%20Reference) (OtherComp :type Primitive%20Component%20Object%20Reference) (OtherBodyIndex :type Integer) (bFromSweep :type Boolean) (SweepResult :type Hit%20Result%20Structure%20%28by%20ref%29))
  (Math|Integer|IncrementInt (Variables|Default|GetEntitiesInCollision)
    (:%20%20
      (CallFunction|Open))))

(event OnComponentEndOverlap(Box)
  (params (OverlappedComponent :type Primitive%20Component%20Object%20Reference) (OtherActor :type Actor%20Object%20Reference) (OtherComp :type Primitive%20Component%20Object%20Reference) (OtherBodyIndex :type Integer))
  (Math|Integer|DecrementInt (Variables|Default|GetEntitiesInCollision)
    (:%20%20
      (CallFunction|Close))))

(event Custom|Open
  (bind _portcullis (Variables|Default|Getportcullis))
  (bind _returnvalue (Transformation|GetWorldLocation _portcullis))
  (bind (_x _y) (Math|Vector|BreakVector _returnvalue))
  (Utilities|FlowControl|DoOnce false
    (:Completed
      (bind _rotation (Timeline|OpenAnimation PlayFromStart)
        (:Update
          (Transformation|SetWorldLocation (Variables|Default|Getportcullis) (Math|Vector|MakeVector _x _y (* _rotation (Math|Conversions|ToFloat(Integer) (Variables|Default|GetTransformDirection)) (Variables|Default|GetHeight))) false false))))))

(event Custom|Close
  (bind _portcullis (Variables|Default|Getportcullis))
  (bind _portcullis_2 (Variables|Default|Getportcullis))
  (bind _returnvalue (Transformation|GetWorldLocation _portcullis_2))
  (bind _returnvalue_2 (Transformation|GetWorldLocation _portcullis))
  (bind (_x _y) (Math|Vector|BreakVector _returnvalue))
  (bind (_x_2 _y_2) (Math|Vector|BreakVector _returnvalue_2))
  (if (== (Variables|Default|GetEntitiesInCollision) 0)
    (Utilities|FlowControl|Sequence
      (:then_0
        (Utilities|FlowControl|DoOnce false) ; enters at Reset
      )
      (:then_1
        (bind _rotation (Timeline|CloseAnimation PlayFromStart)
          (:Update
            (Transformation|SetWorldLocation (Variables|Default|Getportcullis) (Math|Vector|MakeVector _x_2 _y_2 (* _rotation (Math|Conversions|ToFloat(Integer) (Variables|Default|GetTransformDirection)) (Variables|Default|GetHeight))) false false)))))))

(event EventBeginPlay)

(event Collision|EventActorBeginOverlap
  (params (OtherActor :type Actor%20Object%20Reference)))

(event EventTick
  (params (DeltaSeconds :type Float%20%28single-precision%29)))

(fn ConstructionScript)