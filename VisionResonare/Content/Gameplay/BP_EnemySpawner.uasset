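; Enemy spawner that runs three escalating waves of werewolf AI, then opens the StartScreen level.
; Once StartSpawn is set, Tick switches on WaveCounter through a delay, and DoOnce gates start each wave with an announcer sound.
; Each wave loops a random delay, spawn and count check, pausing before the next wave.
; Spawn points are picked randomly from three, but the third wave always spawns at SpawnLocation, ignoring the pick.
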(event EventBeginPlay
  ;[1 1 1] Enemy Spawner(by Patrick Kokozka)
  (Variables|Default|SetEnemies%20Counter 0))

(event EventTick
  (params (DeltaSeconds :type Float%20%28single-precision%29))
  ;[1 1 1] Enemy Spawner(by Patrick Kokozka)
  (Utilities|FlowControl|Sequence
    (:then_0
      (if (Variables|Default|GetStartSpawn)
        (Utilities|FlowControl|Delay 2.0)
        (switch int (Variables|Default|GetWaveCounter)
          (:0
            (Utilities|FlowControl|DoOnce false
              (:Completed
                (Audio|PlaySound2D "/Game/Sound/EnemyCounter/S_1One.S_1One" 1.0 1.0 0.0 0 0)
                (Utilities|FlowControl|Delay (Math|Random|RandomFloatinRange (Variables|Default|GetMinRespawnTime) (Variables|Default|GetMaxRespawnTime)) :!label _label)
                (AI|SpawnAIFromClass "/Game/Characters/Werewolf/Blueprints/BP_Werewolf.BP_Werewolf_C" "/Game/Characters/Werewolf/AI/Werewolf_BT.Werewolf_BT" (Variables|Default|GetTempLocation) "0, 0, 0" false)
                (bind _output_get (Variables|Default|SetFirstWave (+ (Variables|Default|GetFirstWave) 1)))
                (if (>= _output_get 5)
                  (Utilities|FlowControl|Delay (Variables|Default|GetWaveRestartTime))
                  (Variables|Default|SetWaveCounter 1)
                  (else
                    (switch int (Math|Random|RandomIntegerinRange 1 3)
                      (:0
                        _)
                      (:1
                        (Variables|Default|SetTempLocation (Variables|Default|GetSpawnLocation2))
                        (goto _label))
                      (:2
                        (Variables|Default|SetTempLocation (Variables|Default|GetSpawnLocation3))
                        (goto _label))
                      (:3
                        _))
                    (Variables|Default|SetTempLocation (Variables|Default|GetSpawnLocation))
                    (goto _label))))))
          (:1
            (Utilities|FlowControl|DoOnce false
              (:Completed
                (Audio|PlaySound2D "/Game/Sound/EnemyCounter/S_2Two.S_2Two" 1.0 1.0 0.0 0 0)
                (Utilities|FlowControl|Delay (Math|Random|RandomFloatinRange (Variables|Default|GetMinRespawnTime) (Variables|Default|GetMaxRespawnTime)) :!label _label_2)
                (AI|SpawnAIFromClass "/Game/Characters/Werewolf/Blueprints/BP_Werewolf.BP_Werewolf_C" "/Game/Characters/Werewolf/AI/Werewolf_BT.Werewolf_BT" (Variables|Default|GetTempLocation) "0, 0, 0" false)
                (bind _output_get_2 (Variables|Default|SetSecondWave (+ (Variables|Default|GetSecondWave) 1)))
                (if (>= _output_get_2 10)
                  (Utilities|FlowControl|Delay (Variables|Default|GetWaveRestartTime))
                  (Variables|Default|SetWaveCounter 2)
                  (else
                    (switch int (Math|Random|RandomIntegerinRange 1 3)
                      (:0
                        _)
                      (:1
                        (Variables|Default|SetTempLocation (Variables|Default|GetSpawnLocation2))
                        (goto _label_2))
                      (:2
                        (Variables|Default|SetTempLocation (Variables|Default|GetSpawnLocation3))
                        (goto _label_2))
                      (:3
                        _))
                    (Variables|Default|SetTempLocation (Variables|Default|GetSpawnLocation))
                    (goto _label_2))))))
          (:2
            (Utilities|FlowControl|DoOnce false
              (:Completed
                (Audio|PlaySound2D "/Game/Sound/EnemyCounter/S_3Three.S_3Three" 1.0 1.0 0.0 0 0)
                (Utilities|FlowControl|Delay (Math|Random|RandomFloatinRange (Variables|Default|GetMinRespawnTime) (Variables|Default|GetMaxRespawnTime)) :!label _label_3)
                (AI|SpawnAIFromClass "/Game/Characters/Werewolf/Blueprints/BP_Werewolf.BP_Werewolf_C" "/Game/Characters/Werewolf/AI/Werewolf_BT.Werewolf_BT" (Variables|Default|GetSpawnLocation) "0, 0, 0" false)
                (bind _output_get_3 (Variables|Default|SetThirdWave (+ (Variables|Default|GetThirdWave) 1)))
                (if (>= _output_get_3 15)
                  (Utilities|FlowControl|Delay (Variables|Default|GetWaveRestartTime))
                  (Variables|Default|SetWaveCounter 3)
                  (else
                    (switch int (Math|Random|RandomIntegerinRange 1 3)
                      (:0
                        _)
                      (:1
                        (Variables|Default|SetTempLocation (Variables|Default|GetSpawnLocation2))
                        (goto _label_3))
                      (:2
                        (Variables|Default|SetTempLocation (Variables|Default|GetSpawnLocation3))
                        (goto _label_3))
                      (:3
                        _))
                    (Variables|Default|SetTempLocation (Variables|Default|GetSpawnLocation))
                    (goto _label_3))))))
          (:3
            (Game|OpenLevel(byName) "StartScreen")))))
    (:then_1
      (if (== (Variables|Default|GetWaveCounter) 3)
        _))))

(event Collision|EventActorBeginOverlap
  (params (OtherActor :type Actor%20Object%20Reference)))

(fn ConstructionScript)