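; Enemy counter actor that announces the count with voice-style number sounds and ends the level at ten.
; It resets EnemiesCounter on BeginPlay and only reads it afterwards, so any increments come from outside this Blueprint.
; Tick feeds a two-second Delay into a switch on the counter, with a DoOnce per value so each sound plays once.
; Reaching ten plays the last sound, waits briefly, then opens MainMenu.
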(event EventBeginPlay
  ;[1 1 1] Enemy Counter (by Patrick Kokozka)
  (Variables|Default|SetEnemies%20Counter 0))

(event EventTick
  (params (DeltaSeconds :type Float%20%28single-precision%29))
  ;[1 1 1] Enemy Counter (by Patrick Kokozka)
  (Utilities|FlowControl|Delay 2.0)
  (switch int (Variables|Default|GetEnemies%20Counter)
    (:0
      (Utilities|FlowControl|DoOnce false))
    (:1
      (Utilities|FlowControl|DoOnce false
        (:Completed
          (Audio|PlaySound2D "/Game/Sound/EnemyCounter/S_1One.S_1One" 1.0 1.0 0.0 0 0))))
    (:2
      (Utilities|FlowControl|DoOnce false
        (:Completed
          (Audio|PlaySound2D "/Game/Sound/EnemyCounter/S_2Two.S_2Two" 1.0 1.0 0.0 0 0))))
    (:3
      (Utilities|FlowControl|DoOnce false
        (:Completed
          (Audio|PlaySound2D "/Game/Sound/EnemyCounter/S_3Three.S_3Three" 1.0 1.0 0.0 0 0))))
    (:4
      (Utilities|FlowControl|DoOnce false
        (:Completed
          (Audio|PlaySound2D "/Game/Sound/EnemyCounter/S_4Four.S_4Four" 1.0 1.0 0.0 0 0))))
    (:5
      (Utilities|FlowControl|DoOnce false
        (:Completed
          (Audio|PlaySound2D "/Game/Sound/EnemyCounter/S_5Five.S_5Five" 1.0 1.0 0.0 0 0))))
    (:6
      (Utilities|FlowControl|DoOnce false
        (:Completed
          (Audio|PlaySound2D "/Game/Sound/EnemyCounter/S_6Six.S_6Six" 1.0 1.0 0.0 0 0))))
    (:7
      (Utilities|FlowControl|DoOnce false
        (:Completed
          (Audio|PlaySound2D "/Game/Sound/EnemyCounter/S_7Seven.S_7Seven" 1.0 1.0 0.0 0 0))))
    (:8
      (Utilities|FlowControl|DoOnce false
        (:Completed
          (Audio|PlaySound2D "/Game/Sound/EnemyCounter/S_8Eight.S_8Eight" 1.0 1.0 0.0 0 0))))
    (:9
      (Utilities|FlowControl|DoOnce false
        (:Completed
          (Audio|PlaySound2D "/Game/Sound/EnemyCounter/S_9Nine.S_9Nine" 1.0 1.0 0.0 0 0))))
    (:10
      (Utilities|FlowControl|DoOnce false
        (:Completed
          (Audio|PlaySound2D "/Game/Sound/EnemyCounter/S_10Ten.S_10Ten" 1.0 1.0 0.0 0 0)
          (Utilities|FlowControl|Delay 2.0)
          (Game|OpenLevel(byName) "MainMenu"))))))

(event Collision|EventActorBeginOverlap
  (params (OtherActor :type Actor%20Object%20Reference)))

(fn ConstructionScript)