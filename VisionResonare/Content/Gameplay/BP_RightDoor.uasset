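; BP_RightDoor is a door actor that swings open when something overlaps its Box and closes after it empties.
; An overlap counter tracks occupants, and a DoOnce stops repeated openings until a close resets it.
; Each exit restarts a four-second retriggerable delay, after which the door closes only if the count is zero.
; Separate open and close timelines set the door's world yaw, scaled by speed and direction variables.
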(event OnComponentBeginOverlap(Box)
  (params (OverlappedComponent :type Primitive%20Component%20Object%20Reference) (OtherActor :type Actor%20Object%20Reference) (OtherComp :type Primitive%20Component%20Object%20Reference) (OtherBodyIndex :type Integer) (bFromSweep :type Boolean) (SweepResult :type Hit%20Result%20Structure%20%28by%20ref%29))
  (Math|Integer|IncrementInt (Variables|Default|GetEntitiesInCollision)
    (:%20%20
      (CallFunction|Open))))

(event OnComponentEndOverlap(Box)
  (params (OverlappedComponent :type Primitive%20Component%20Object%20Reference) (OtherActor :type Actor%20Object%20Reference) (OtherComp :type Primitive%20Component%20Object%20Reference) (OtherBodyIndex :type Integer))
  (Math|Integer|DecrementInt (Variables|Default|GetEntitiesInCollision)
    (:%20%20
      (CallFunction|Close))))

(event Custom|Open
  (Utilities|FlowControl|DoOnce false
    (:Completed
      (bind _rotation (Timeline|OpenAnimation PlayFromStart)
        (:Update
          (Transformation|SetWorldRotation (Variables|Default|GetDoor) (Math|Rotator|MakeRotator 0.0 0.0 (* (Variables|Default|GetRotationSpeed) _rotation (Math|Conversions|ToFloat(Integer) (Variables|Default|GetRotationDirection)))) false false))))))

(event Custom|Close
  (Utilities|FlowControl|RetriggerableDelay 4.0)
  (if (== (Variables|Default|GetEntitiesInCollision) 0)
    (Utilities|FlowControl|Sequence
      (:then_0
        (Utilities|FlowControl|DoOnce false) ; enters at Reset
      )
      (:then_1
        (bind _rotation (Timeline|CloseAnimation PlayFromStart)
          (:Update
            (Transformation|SetWorldRotation (Variables|Default|GetDoor) (Math|Rotator|MakeRotator 0.0 0.0 (* (Variables|Default|GetRotationSpeed) _rotation (Math|Conversions|ToFloat(Integer) (Variables|Default|GetRotationDirection)))) false false)))))))

(event EventBeginPlay)

(event Collision|EventActorBeginOverlap
  (params (OtherActor :type Actor%20Object%20Reference)))

(event EventTick
  (params (DeltaSeconds :type Float%20%28single-precision%29)))

(fn ConstructionScript)