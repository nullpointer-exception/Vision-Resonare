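; Clock actor that shows the local system time with rotating hour and minute hands and a swinging pendulum.
; Tick sets each mesh's relative pitch from Now, taking the hour by splitting the formatted time string at the colon.
; The minute hand adds seconds with the opposite sign to minutes.
; The pendulum follows a sine of the milliseconds scaled by Angle, swinging about once per second.
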(event EventTick
  (params (DeltaSeconds :type Float%20%28single-precision%29))
  (bind _returnvalue (Math|DateTime|Now))
  (bind _returnvalue_2 (Class|KismetMathLibrary|GetMinute _returnvalue))
  (bind _returnvalue_3 (Class|KismetMathLibrary|GetSecond _returnvalue))
  (bind _returnvalue_4 (Math|Conversions|ToFloat(Integer) _returnvalue_3))
  (Transformation|SetRelativeRotation (Variables|Default|GetSM_Hour_hand) (Math|Rotator|MakeRotator 0.0 (* (+ (* (+ (* (Math|Conversions|ToInteger(Byte) (.LeftS (Utilities|String|Split (Utilities|String|ToString(Text) (Class|KismetTextLibrary|AsTimeDateTime _returnvalue)) ":"))) 6e+01) (Math|Conversions|ToFloat(Integer) _returnvalue_2)) 6e+01) _returnvalue_4) -0.008333) 0.0) false false)
  (Transformation|SetRelativeRotation (Variables|Default|GetSM_Minute_hand) (Math|Rotator|MakeRotator 0.0 (* (+ _returnvalue_4 (* _returnvalue_2 -6e+01)) 0.1) 0.0) false false)
  (Transformation|SetRelativeRotation (Variables|Default|GetSM_Pendulum) (Math|Rotator|MakeRotator 0.0 (* (Math|Trig|Sin(Degrees) (/ (Math|Conversions|ToFloat(Integer) (Math|DateTime|GetMillisecond _returnvalue)) 2.8)) (Variables|Default|GetAngle)) 0.0) false false))

(fn ConstructionScript)